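; Death ghost hazard actor for the TapGhosts game, which ends the game if the player taps it.
; On spawn it caches the game mode and plays its GhostFloat flipbook once, without looping.
; A touch on the flipbook stops it, calls EndGame on the game mode and destroys the actor.
; If the flipbook finishes untapped, the game mode spawns a normal ghost and decrements its ghosts, and the actor destroys itself.
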(event `self.ReceiveTick`
  (params (DeltaSeconds :type "Float (single-precision)")))

(event `self.ReceiveActorBeginOverlap`
  (params (OtherActor :type "Actor Object Reference")))

(event `self.ReceiveBeginPlay`
  ;[1 1 1] Spawn death and play its flipbook
  (bind _astap_ghosts_game_mode (cast `/Game/TapGhostsGameMode` (`GameplayStatics.GetGameMode`)))
  (set `self.GameMode_0` _astap_ghosts_game_mode)
  (`PaperFlipbookComponent.SetLooping` (`self.GhostFloat`) false)
  (`PaperFlipbookComponent.PlayFromStart` (`self.GhostFloat`)))

(event `self.GhostFloat.OnInputTouchBegin`
  (params (FingerIndex :type "ETouchIndex Enum" :default "Touch1") (TouchedComponent :type "PrimitiveComponent Object Reference"))
  ;[1 1 1] Player has tapped death ghost, game over
  (`PaperFlipbookComponent.Stop` (`self.GhostFloat`))
  (`/Game/TapGhostsGameMode.EndGame` (`self.GameMode_0`))
  (`self.K2_DestroyActor`))

(event `self.GhostFloat.OnFinishedPlaying`
  ;[1 1 1] Death has passed with no tap, spawn normal ghost
  (`/Game/TapGhostsGameMode.SpawnGhost` (`self.GameMode_0`))
  (`/Game/TapGhostsGameMode.DecrementGhosts` (`self.GameMode_0`))
  (`self.K2_DestroyActor`))

(fn `UserConstructionScript`
  (`parent.UserConstructionScript`))