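; GhostBP is a tappable ghost for a Tap Ghosts game, drawn as a randomly chosen flipbook that plays once on spawn.
; If the animation finishes untapped, it tells the game mode to cut the score.
; A touch stops the animation, adds score and combo, spawns another mob and emits sparkles at the arrow.
; Both outcomes decrement the game mode's ghost count and destroy the actor.
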(event `self.ReceiveActorBeginOverlap`
  (params (OtherActor :type "Actor Object Reference")))

(event `self.ReceiveTick`
  (params (DeltaSeconds :type "Float (single-precision)")))

(event `self.ReceiveBeginPlay`
  (bind _ghostanims (`self.GhostAnims`))
  (bind _ghostfloat (`self.GhostFloat`))
  ;[1 1 1] Spawn ghost and play its flipbook
  (bind _astap_ghosts_game_mode (cast `/Game/TapGhostsGameMode` (`GameplayStatics.GetGameMode`)))
  (set `self.GameMode` _astap_ghosts_game_mode)
  (`PaperFlipbookComponent.SetFlipbook` _ghostfloat (`KismetArrayLibrary.Array_Get` _ghostanims (`KismetMathLibrary.RandomIntegerInRange` 0 (`KismetArrayLibrary.Array_LastIndex` _ghostanims))))
  (`PaperFlipbookComponent.SetLooping` _ghostfloat false)
  (`PaperFlipbookComponent.PlayFromStart` (`self.GhostFloat`)))

(event `self.GhostFloat.OnFinishedPlaying`
  (bind _gamemode (`self.GameMode`))
  ;[1 1 1] Ghost has died, cut player score
  (`/Game/TapGhostsGameMode.CutScore` _gamemode)
  (`/Game/TapGhostsGameMode.DecrementGhosts` _gamemode :!label _label)
  (`self.K2_DestroyActor`))

(event `self.GhostFloat.OnInputTouchBegin`
  (params (FingerIndex :type "ETouchIndex Enum" :default "Touch1") (TouchedComponent :type "PrimitiveComponent Object Reference"))
  (bind _gamemode (`self.GameMode`))
  ;[1 1 1] Ghost was tapped, addscore, combo and spawn another mob
  (`PaperFlipbookComponent.Stop` (`self.GhostFloat`))
  (`/Game/TapGhostsGameMode.AddScore` (`self.GameMode`) (`self.GhostValue`))
  (`/Game/TapGhostsGameMode.SpawnMob` _gamemode)
  (`/Game/TapGhostsGameMode.AddCombo` _gamemode)
  (`|SpawnActorFromClass` "/Game/Blueprints/SparklesBP.SparklesBP_C" (`SceneComponent.K2_GetComponentToWorld` (`self.Arrow`)) "Undefined" "OverrideRootScale")
  (goto _label))

(fn `UserConstructionScript`)