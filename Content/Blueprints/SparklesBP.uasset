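; SparklesBP is a one-shot sparkle effect actor for what appears to be the Tap Ghosts game.
; On BeginPlay it plays its Sparkles component once without looping, then destroys itself when playback finishes.
; It also checks the game instance's sound setting, but that branch does nothing, as the delayed, volume-scaled UI sound is disconnected and never runs.
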(event `self.ReceiveBeginPlay`
  (bind _sparkles (`self.Sparkles`))
  (`PaperFlipbookComponent.SetLooping` _sparkles false)
  (`PaperFlipbookComponent.PlayFromStart` _sparkles)
  (bind _astap_ghosts_game_instance (cast `/Game/TapGhostsGameInstance` (`GameplayStatics.GetGameInstance`)))
  (if (`/Game/TapGhostsGameInstance.SoundEnabled` _astap_ghosts_game_instance)
    _))

(event `self.ReceiveActorBeginOverlap`
  (params (OtherActor :type "Actor Object Reference")))

(event `self.ReceiveTick`
  (params (DeltaSeconds :type "Float (single-precision)")))

(event `self.Sparkles.OnFinishedPlaying`
  (`self.K2_DestroyActor`))

(fn `UserConstructionScript`)